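; Base character Blueprint that manages an equipped weapon, ability activation and combat reactions.
; BeginPlay equips the current weapon definition, then activates melee-tagged abilities after a short delay.
; EquipWeapon caches spawned weapons in a pool keyed by definition identifier, reusing them and attaching to the mesh's sword socket.
; Combat interface events toggle weapon collision and play hit reactions, while helper checks report health, pause and active-skill state.
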(event EventAttackStart
  ;[1 1 1] ICombat
  (Default|EnableCollision (Variables|Combat|GetCurrentWeapon)))

(event EventAttackEnd
  ;[1 1 1] ICombat
  (Default|DisableCollision (Variables|Combat|GetCurrentWeapon)))

(event EventDamageTaken
  ;[1 1 1] ICombat
  (Animation|PlayAnimMontage (Variables|Combat|GetHitReactMontage) 1.0 "None"))

(event EventBeginPlay
  (CallFunction|EquipWeapon (Variables|Default|GetCurrentWeaponDefinition))
  (Utilities|FlowControl|Delay 0.5)
  (Class|GameDevGameJamCharacter|ActivateAbilitieswithTags "(GameplayTags=((TagName=\"Ability.Melee\")))" true))

(fn ConstructionScript)

(fn EquipWeapon
  (params (WeaponDef :type Weapon%20Definition%20Object%20Reference%20%28by%20ref%29))
  (bind _returnvalue (Class|ItemDefinition|GetIdentifierString WeaponDef))
  (bind _weaponpool (Variables|Combat|GetWeaponPool))
  (bind (_value _returnvalue_2) (Utilities|Map|Find _weaponpool _returnvalue))
  (Utilities|IsValid (Variables|Combat|GetCurrentWeapon)
    (:Is%20Valid
      (Transformation|DetachFromActor (Variables|Combat|GetCurrentWeapon) "KeepRelative" "KeepRelative" "KeepRelative"))
    (:Is%20Not%20Valid
      _))
  (Utilities|IsValid WeaponDef
    (:Is%20Valid
      (bind _asweapon_base (Utilities|Casting|CastToWeaponBaseClass (Variables|/Script/GameDevGameJam.WeaponDefinition|GetWeaponActor WeaponDef))
        (:then
          (Variables|Default|SetCurrentWeaponDefinition WeaponDef)
          (if _returnvalue_2
            (Variables|Combat|SetCurrentWeapon _value)
            (else
              (bind _returnvalue_3 (Game|SpawnActorfromClass _asweapon_base (Math|Transform|MakeTransform "0, 0, 0") "Undefined" 0 0))
              (bind _output_get (Variables|Combat|SetCurrentWeapon _returnvalue_3))
              (Utilities|Map|Add _weaponpool _returnvalue _output_get)))
          (Transformation|AttachComponentToComponent (Variables|Combat|GetCurrentWeapon) (Variables|Character|GetMesh) "Sword" "KeepRelative" "KeepRelative" "KeepRelative" true))
        (:CastFailed
          (Development|PrintString "Not a WeaponBase Class!"))))
    (:Is%20Not%20Valid
      (Development|PrintString "Not a WeaponDef"))))

(fn UnequipWeapon
  (Utilities|IsValid (Variables|Combat|GetCurrentWeapon)
    (:Is%20Valid
      (Transformation|DetachFromActor (Variables|Combat|GetCurrentWeapon) "KeepRelative" "KeepRelative" "KeepRelative")
      (Variables|Combat|SetCurrentWeapon 0)
      (Variables|Default|SetCurrentWeaponDefinition 0))
    (:Is%20Not%20Valid
      (Development|PrintString "no sword to detach"))))

(fn CanUseAnyAbility
  (return (Math|Boolean|ANDBoolean (CallFunction|IsAlive) (not (Game|IsGamePaused)) (not (CallFunction|IsUsingSkill)))))

(fn IsAlive
  (return (> (Class|GameDevGameJamCharacter|GetHealth) 0.0)))

(fn IsUsingSkill
  (bind _activeabilities (Class|GameDevGameJamCharacter|GetActiveAbilitieswithTags "(GameplayTags=((TagName=\"Ability.Skill\")))"))
  (return (> (Utilities|Array|Length _activeabilities) 0)))